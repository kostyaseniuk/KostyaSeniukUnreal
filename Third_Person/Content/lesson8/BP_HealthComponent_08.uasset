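; BP_HealthComponent_08 is a lesson 8 health component that tracks a Health value.
; AddHealth raises Health and AddDamage lowers it by fixed amounts, with no clamping, then each prints the new value on screen in green or red respectively.
; GetHealth is an empty stub, and the event graph holds only disabled default events.
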(event EventBeginPlay)

(event EventTick
  (params (DeltaSeconds :type Float%20%28single-precision%29)))

(fn AddHealth
  (Variables|Default|SetHealth (+ (Variables|Default|GetHealth) 3.0))
  (Development|PrintString (Utilities|String|ToString(Float) (Variables|Default|GetHealth)) true true "(R=0.017680,G=1.000000,B=0.086371,A=1.000000)" 1e+01))

(fn AddDamage
  (Variables|Default|SetHealth (- (Variables|Default|GetHealth) 8.0))
  (Development|PrintString (Utilities|String|ToString(Float) (Variables|Default|GetHealth)) true true "(R=1.000000,G=0.055524,B=0.165213,A=1.000000)" 1e+01))

(fn GetHealth)