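; BP_Patrol_AIControler_10 is an AI controller that sets up a two-point patrol for its pawn.
; On BeginPlay it runs the BT_Patrol_10 behavior tree, then seeds the blackboard with PointA, PointB and DelayTime.
; Both points are fixed, opposite offsets from the first player controller's own actor location, sampled at startup rather than tracked.
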(event EventBeginPlay
  (bind _returnvalue (Game|GetPlayerController 0))
  (bind _blackboard1 (Variables|Default|GetBlackboard1))
  (bind _returnvalue_2 (Transformation|GetActorLocation _returnvalue))
  (AI|RunBehaviorTree "/Game/lesson10_AI-Сontrolle/BT_Patrol_10.BT_Patrol_10")
  (AI|Components|Blackboard|SetValueasVector _blackboard1 (Variables|Default|GetPointA) (+ _returnvalue_2 "200.000000,100.000000,0.000000"))
  (AI|Components|Blackboard|SetValueasVector _blackboard1 (Variables|Default|GetPointB) (+ _returnvalue_2 "-200.000000,-100.000000,0.000000"))
  (AI|Components|Blackboard|SetValueasFloat _blackboard1 (Variables|Default|GetDelayTime) 5e+01))

(fn ConstructionScript)